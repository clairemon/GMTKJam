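; SuspensionComponent is a raycast hover-suspension component that pushes a physics-simulated parent mesh away from surfaces below it.
; InitComponent stores the given mesh and enables physics on it.
; Each Tick traces along its negative up vector, then applies force at its own location along the impact normal, fading linearly with hit distance.
; A hit also raises linear and angular damping, which is never reset here.
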(event Custom|InitComponent
  (params (MeshComponent :type Static%20Mesh%20Component%20Object%20Reference))
  (bind _output_get (Variables|Default|SetParentComponent MeshComponent))
  (Physics|SetSimulatePhysics _output_get true))

(event EventTick
  (params (DeltaSeconds :type Float%20%28single-precision%29))
  (bind _returnvalue (Transformation|GetWorldLocation))
  (bind _returnvalue_2 (Math|Vector|GetUpVector))
  (bind _tracelength (Variables|Default|GetTraceLength))
  (bind _parentcomponent (Variables|Default|GetParentComponent))
  (bind _returnvalue_3 (* _tracelength -1.0))
  (bind _returnvalue_4 (* _returnvalue_2 _returnvalue_3))
  (bind _returnvalue_5 (+ _returnvalue _returnvalue_4))
  (Variables|Default|SetHitLocation _returnvalue_5)
  (bind (_outhit _returnvalue_6) (Collision|LineTraceByChannel _returnvalue _returnvalue_5 "TraceTypeQuery1" false 0 "ForOneFrame"))
  (if _returnvalue_6
    (Variables|Default|SetHitLocation (.Location (Collision|BreakHitResult _outhit)))
    (Class|PrimitiveComponent|AddForceatLocation _parentcomponent (* (.ImpactNormal (Collision|BreakHitResult _outhit)) (Math|Float|Lerp (Variables|Default|GetHoverForce) 0.0 (/ (.Distance (Collision|BreakHitResult _outhit)) (Variables|Default|GetTraceLength)))) (Transformation|GetWorldLocation) "None")
    (Class|PrimitiveComponent|SetLinearDamping _parentcomponent 3.0)
    (Class|PrimitiveComponent|SetAngularDamping _parentcomponent 1e+01)))