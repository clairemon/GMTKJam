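; Passenger Blueprint that cycles idle waiting animations on its CrashReactPass01 mesh.
; BeginPlay plays the first waiting animation and starts a looping five-second timer.
; Each timer tick runs a FlipFlop that alternates the two non-looping animations, starting with the first again.
; The construction script only assigns Destination to itself, and nothing else in the graphs uses it.
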(event Custom|Animations
  (bind _crashreactpass01 (Variables|Default|GetCrashReactPass01))
  (Utilities|FlowControl|FlipFlop
    (:A
      (Components|Animation|PlayAnimation _crashreactpass01 "/Game/Animations/Passenger/Waiting01_Anim.Waiting01_Anim" false))
    (:B
      (Components|Animation|PlayAnimation _crashreactpass01 "/Game/Animations/Passenger/Waiting02_Anim.Waiting02_Anim" false))))

(event EventBeginPlay
  (Components|Animation|PlayAnimation (Variables|Default|GetCrashReactPass01) "/Game/Animations/Passenger/Waiting01_Anim.Waiting01_Anim" false)
  (Utilities|Time|SetTimerbyEvent (delegate Custom|Animations) 5.0 true))

(fn ConstructionScript
  (Variables|Default|SetDestination (Variables|Default|GetDestination)))