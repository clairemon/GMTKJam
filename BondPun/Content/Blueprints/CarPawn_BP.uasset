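; Player car pawn for a passenger-delivery game that always drives forward, steering by torque with a handbrake drift turn speed.
; Four suspension components carry the mesh, while a downward impulse fakes gravity.
; A looping timer randomly fires gadgets: speed thruster, steering-locking ice beam, suspension-stretching stilts, or an ejector seat demanding a three-second rescue.
; Tag-based box overlaps handle bounces, pickups, drop-offs and rescues, with a cone pointing at the current destination.
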(event OnComponentBeginOverlap(Box)
  (params (OverlappedComponent :type Primitive%20Component%20Object%20Reference) (OtherActor :type Actor%20Object%20Reference) (OtherComp :type Primitive%20Component%20Object%20Reference) (OtherBodyIndex :type Integer) (bFromSweep :type Boolean) (SweepResult :type Hit%20Result%20Structure%20%28by%20ref%29))
  (bind _carmesh (Variables|Default|GetCarMesh))
  (bind _returnvalue (Math|Vector|GetForwardVector _carmesh))
  (bind _returnvalue_2 (* (Math|Vector|MakeVector (.x _returnvalue) (.y _returnvalue) 0.0) 3e+05))
  (bind _returnvalue_3 (* _returnvalue_2 -1.0))
  ;[1 1 1] Detect what player hits
  (if (Actor|ActorHasTag OtherActor "Bouncy")
    (Physics|AddImpulse (Variables|Default|GetCarMesh) (Math|Vector|MakeVector (.x _returnvalue_3) (.y _returnvalue_3) 0.0) "None" false)
    (elif (Actor|ActorHasTag OtherActor "Passenger")
      (bind _aspassenger_bp (Utilities|Casting|CastToPassenger_BP OtherActor))
      (bind _output_get (Variables|Default|SetPassengerDestination (Variables|/Game/Blueprints/Passenger_BP.Passenger_BP_C|GetDestination _aspassenger_bp)))
      (Variables|Default|SetCurrentDestination _output_get)
      (Variables|Default|SetHasPassenger true)
      (Utilities|IsValid _aspassenger_bp
        (:Is%20Valid
          (Actor|DestroyActor _aspassenger_bp)
          (bind _returnvalue_4 (Game|SpawnActorfromClass "/Game/Blueprints/Destination_BP.Destination_BP_C" (Math|Transform|MakeTransform (Variables|Default|GetCurrentDestination) "0, 0, 0" "1,1,1") "Undefined" 0 0))
          (Variables|Default|SetCurrentDestinationBP _returnvalue_4)))
      (elif (Actor|ActorHasTag OtherActor "Destination")
        (Actor|DestroyActor OtherActor)
        (Development|PrintString "Reached Destination!")
        (Variables|Default|SetHasPassenger false)
        (elif (Actor|ActorHasTag OtherActor "EDestination")
          (Actor|DestroyActor OtherActor)
          (Variables|Default|SetCurrentDestination (Variables|Default|GetPassengerDestination))
          (Development|PrintString "You saved the passenger!"))))))

(event Custom|ActivateStilts
  (bind _suspensioncomponent_bp (Variables|Default|GetSuspensionComponent_BP))
  (bind _suspensioncomponent_bp1 (Variables|Default|GetSuspensionComponent_BP1))
  (bind _suspensioncomponent_bp2 (Variables|Default|GetSuspensionComponent_BP2))
  (bind _suspensioncomponent_bp3 (Variables|Default|GetSuspensionComponent_BP3))
  (bind _jumpheight (Variables|Default|GetJumpHeight))
  (bind _returnvalue (/ 1.0 _jumpheight))
  ;[1 1 1] Activate Stilts
  (Utilities|FlowControl|DoOnce false :!label _label
    (:Completed
      (Variables|Default|SetStiltsOn true)
      (Variables|/Game/Blueprints/SuspensionComponent_BP.SuspensionComponent_BP_C|SetTraceLength _suspensioncomponent_bp (* _jumpheight (Variables|/Game/Blueprints/SuspensionComponent_BP.SuspensionComponent_BP_C|GetTraceLength _suspensioncomponent_bp)))
      (Variables|/Game/Blueprints/SuspensionComponent_BP.SuspensionComponent_BP_C|SetTraceLength _suspensioncomponent_bp1 (* _jumpheight (Variables|/Game/Blueprints/SuspensionComponent_BP.SuspensionComponent_BP_C|GetTraceLength _suspensioncomponent_bp1)))
      (Variables|/Game/Blueprints/SuspensionComponent_BP.SuspensionComponent_BP_C|SetTraceLength _suspensioncomponent_bp2 (* _jumpheight (Variables|/Game/Blueprints/SuspensionComponent_BP.SuspensionComponent_BP_C|GetTraceLength _suspensioncomponent_bp2)))
      (Variables|/Game/Blueprints/SuspensionComponent_BP.SuspensionComponent_BP_C|SetTraceLength _suspensioncomponent_bp3 (* _jumpheight (Variables|/Game/Blueprints/SuspensionComponent_BP.SuspensionComponent_BP_C|GetTraceLength _suspensioncomponent_bp3)))
      (Utilities|FlowControl|Delay 5.0)
      (Variables|/Game/Blueprints/SuspensionComponent_BP.SuspensionComponent_BP_C|SetTraceLength _suspensioncomponent_bp (* (Variables|/Game/Blueprints/SuspensionComponent_BP.SuspensionComponent_BP_C|GetTraceLength _suspensioncomponent_bp) _returnvalue))
      (Variables|/Game/Blueprints/SuspensionComponent_BP.SuspensionComponent_BP_C|SetTraceLength _suspensioncomponent_bp1 (* (Variables|/Game/Blueprints/SuspensionComponent_BP.SuspensionComponent_BP_C|GetTraceLength _suspensioncomponent_bp1) _returnvalue))
      (Variables|/Game/Blueprints/SuspensionComponent_BP.SuspensionComponent_BP_C|SetTraceLength _suspensioncomponent_bp2 (* (Variables|/Game/Blueprints/SuspensionComponent_BP.SuspensionComponent_BP_C|GetTraceLength _suspensioncomponent_bp2) _returnvalue))
      (Variables|/Game/Blueprints/SuspensionComponent_BP.SuspensionComponent_BP_C|SetTraceLength _suspensioncomponent_bp3 (* (Variables|/Game/Blueprints/SuspensionComponent_BP.SuspensionComponent_BP_C|GetTraceLength _suspensioncomponent_bp3) _returnvalue))
      (Variables|Default|SetStiltsOn false)
      (goto _label Reset))))

(event Custom|GoForward
  (bind _carmesh (Variables|Default|GetCarMesh))
  (bind _carspeed (Variables|Default|GetCarSpeed))
  (bind _returnvalue (Math|Vector|GetForwardVector _carmesh))
  (bind _returnvalue_2 (* (Math|Vector|MakeVector (.x _returnvalue) (.y _returnvalue) 0.0) _carspeed))
  (bind _returnvalue_3 (* _returnvalue_2 1.0))
  ;[1 1 1] Go Forward (Always happening)
  (Physics|AddForce (Variables|Default|GetCarMesh) (Math|Vector|MakeVector (.x _returnvalue_3) (.y _returnvalue_3) 0.0) "None" false))

(event Custom|AddGravity
  (bind _carmesh (Variables|Default|GetCarMesh))
  (bind _returnvalue (Transformation|GetWorldLocation _carmesh))
  ;[1 1 1] Add artificial gravity
  (bind _outhit (Collision|LineTraceByChannel (Math|Vector|MakeVector (.x _returnvalue) (.y _returnvalue) (.z _returnvalue)) (Math|Vector|MakeVector (.x _returnvalue) (.y _returnvalue) 0.0) "TraceTypeQuery1" false 0 "ForOneFrame"))
  (if (> (.Distance (Collision|BreakHitResult _outhit)) 1e+02)
    (if (not (Variables|Default|GetStiltsOn))
      (Physics|AddImpulse (Variables|Default|GetCarMesh) "0, 0,-1000.000000" "None" false))))

(event Custom|Thruster
  ;[1 1 1] Thruster
  (bind _output_get (Variables|Default|SetCarSpeed (* (Variables|Default|GetCarSpeed) 2.0)))
  (Utilities|FlowControl|Delay 5.0)
  (Variables|Default|SetCarSpeed (* _output_get 0.5)))

(event Custom|PointTowardsDestination
  (bind _carmesh (Variables|Default|GetCarMesh))
  (bind _currentdestination (Variables|Default|GetCurrentDestination))
  (bind _returnvalue (Transformation|GetWorldLocation _carmesh))
  (bind _returnvalue_2 (Math|Rotator|FindLookatRotation _returnvalue _currentdestination))
  ;[1 1 1] Control arrow pointing
  (if (Variables|Default|GetHasPassenger)
    (Rendering|SetVisibility (Variables|Default|GetCone) true false)
    (Transformation|SetWorldRotation (Variables|Default|GetCone) (Math|Rotator|MakeRotator (.roll _returnvalue_2) (- (.pitch _returnvalue_2) 9e+01) (.yaw _returnvalue_2)) false false)
    (else
      (Rendering|SetVisibility (Variables|Default|GetCone) false false))))

(event Custom|IceBeam
  (bind _returnvalue (Game|GetPlayerController 0))
  ;[1 1 1] IceBeam
  (bind _output_get (Variables|Default|SetSavedTurning (Variables|Default|GetTurningValue)))
  (Input|DisableInput _returnvalue)
  (Variables|Default|SetTurningValue _output_get)
  (Utilities|FlowControl|Delay 4.0)
  (Input|EnableInput _returnvalue))

(event Custom|AddTorque
  ;[1 1 1] Turn Control
  (Class|PrimitiveComponent|AddTorqueinDegrees (Variables|Default|GetCarMesh) (Math|Vector|MakeVector 0.0 0.0 (* (Variables|Default|GetTurningValue) (* (Variables|Default|GetTurnSpeed) 1e+06))) "None" false))

(event Custom|Random%20gadget
  (switch int (Math|Random|RandomIntegerinRange 0 11)
    (:0
      (CallFunction|Thruster :!label _label)
      (Development|PrintString "THRUSTER ACTIVATED"))
    (:1
      (goto _label))
    (:2
      (CallFunction|IceBeam :!label _label_2)
      (Development|PrintString "ICE BEAM ACTIVATED"))
    (:3
      (goto _label_2))
    (:4
      (CallFunction|ActivateStilts :!label _label_3)
      (Development|PrintString "STILTS ACTIVATED"))
    (:5
      (goto _label_3))
    (:6
      (CallFunction|EjectorSeat)
      (Development|PrintString "EJECTOR SEAT ACTIVATED"))))

(event Custom|EjectorSeat
  (bind _carmesh (Variables|Default|GetCarMesh))
  (bind _returnvalue (Math|Vector|GetForwardVector _carmesh))
  (bind _returnvalue_2 (Transformation|GetWorldLocation _carmesh))
  (bind _returnvalue_3 (* _returnvalue 1e+03))
  (bind _returnvalue_4 (+ _returnvalue_3 _returnvalue_2))
  (if (Variables|Default|GetHasPassenger)
    (bind _output_get (Variables|Default|SetCurrentDestination (Math|Vector|MakeVector (+ (Math|Random|RandomFloatinRange -5e+02 5e+02) (.x _returnvalue_4)) (+ (.y _returnvalue_4) (Math|Random|RandomFloatinRange -5e+02 5e+02)) 0.0)))
    (bind _returnvalue_5 (Game|SpawnActorfromClass "/Game/Blueprints/EjectorDestination_BP.EjectorDestination_BP_C" (Math|Transform|MakeTransform _output_get "0, 0, 0" "1,1,1") "Undefined" 0 0))
    (Utilities|FlowControl|Delay 3.0)
    (Utilities|IsValid _returnvalue_5
      (:Is%20Valid
        (Development|PrintString "Passenger died!")
        (Variables|Default|SetHasPassenger false)
        (Actor|DestroyActor (Variables|Default|GetCurrentDestinationBP))))))

(event EventBeginPlay
  (bind _carmesh (Variables|Default|GetCarMesh))
  (Default|InitComponent (Variables|Default|GetSuspensionComponent_BP) _carmesh)
  (Default|InitComponent (Variables|Default|GetSuspensionComponent_BP1) _carmesh)
  (Default|InitComponent (Variables|Default|GetSuspensionComponent_BP2) _carmesh)
  (Default|InitComponent (Variables|Default|GetSuspensionComponent_BP3) _carmesh)
  (Variables|Default|SetStartingTurnSpeed (Variables|Default|GetTurnSpeed))
  (Utilities|Time|SetTimerbyEvent (delegate Custom|Random%20gadget) (Variables|Default|GetGadgetTimer) true))

(event EventTick
  (params (DeltaSeconds :type Float%20%28single-precision%29))
  (CallFunction|GoForward)
  (CallFunction|AddGravity)
  (CallFunction|PointTowardsDestination)
  (CallFunction|AddTorque))

(event Input|ActionEvents|InputActionHandBrake
  (params (Key :type Key%20Structure :default "None"))
  (:Pressed
    (Variables|Default|SetTurnSpeed (Variables|Default|GetDriftSpeed)))
  (:Released
    (Variables|Default|SetTurnSpeed (Variables|Default|GetStartingTurnSpeed))))

(event Input|ActionEvents|InputActionFlip
  (params (Key :type Key%20Structure :default "None"))
  ;[1 1 1] Flip car right side up
  (:Pressed
    (Transformation|SetWorldRotation (Variables|Default|GetCarMesh) (Math|Rotator|MakeRotator 0.0 0.0 0.0) false false)))

(event Input|ActionEvents|InputActionThruster
  (params (Key :type Key%20Structure :default "None"))
  ;[1 1 1] Debug inputs
  (:Pressed
    (Utilities|FlowControl|DoOnce false :!label _label
      (:Completed
        (CallFunction|Thruster)
        (Utilities|FlowControl|Delay 5.0)
        (goto _label Reset)))))

(event Input|ActionEvents|InputActionStilts
  (params (Key :type Key%20Structure :default "None"))
  ;[1 1 1] Debug inputs
  (:Pressed
    (CallFunction|EjectorSeat)))

(event Input|AxisEvents|InputAxisForward
  (params (AxisValue :type Float%20%28single-precision%29))
  ;[1 1 1] Control for debugging
)

(event Input|AxisEvents|InputAxisTurn
  (params (AxisValue :type Float%20%28single-precision%29))
  ;[1 1 1] Turn Control
  (Variables|Default|SetTurningValue AxisValue))

(fn ConstructionScript)