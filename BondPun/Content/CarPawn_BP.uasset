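; Physics-driven car pawn that constantly drives forward on four trace-based suspension components, steered by yaw torque and bounced back on box overlaps.
; Each tick applies forward force and, when a trace reads over 100 units, extra downward impulse unless stilts are on.
; Timed abilities temporarily lengthen suspension traces (stilts) or double speed (thruster), and a Flip input rights the car.
; The Forward debug input is disconnected, and roll is printed each tick.
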(event OnComponentBeginOverlap(Box)
  (params (OverlappedComponent :type Primitive%20Component%20Object%20Reference) (OtherActor :type Actor%20Object%20Reference) (OtherComp :type Primitive%20Component%20Object%20Reference) (OtherBodyIndex :type Integer) (bFromSweep :type Boolean) (SweepResult :type Hit%20Result%20Structure%20%28by%20ref%29))
  (bind _carmesh (Variables|Default|GetCarMesh))
  (bind _returnvalue (Math|Vector|GetForwardVector _carmesh))
  (bind _returnvalue_2 (* (Math|Vector|MakeVector (.x _returnvalue) (.y _returnvalue) 0.0) 3e+05))
  (bind _returnvalue_3 (* _returnvalue_2 -1.0))
  ;[1 1 1] Bounce back when hitting wall
  (Physics|AddImpulse (Variables|Default|GetCarMesh) (Math|Vector|MakeVector (.x _returnvalue_3) (.y _returnvalue_3) -0.0) "None" false))

(event Custom|ActivateStilts
  (bind _suspensioncomponent_bp (Variables|Default|GetSuspensionComponent_BP))
  (bind _suspensioncomponent_bp1 (Variables|Default|GetSuspensionComponent_BP1))
  (bind _suspensioncomponent_bp2 (Variables|Default|GetSuspensionComponent_BP2))
  (bind _suspensioncomponent_bp3 (Variables|Default|GetSuspensionComponent_BP3))
  (bind _jumpheight (Variables|Default|GetJumpHeight))
  (bind _returnvalue (/ 1.0 _jumpheight))
  ;[1 1 1] Activate Stilts
  (Utilities|FlowControl|DoOnce false :!label _label
    (:Completed
      (Variables|Default|SetStiltsOn true)
      (Variables|/Game/SuspensionComponent_BP.SuspensionComponent_BP_C|SetTraceLength _suspensioncomponent_bp (* _jumpheight (Variables|/Game/SuspensionComponent_BP.SuspensionComponent_BP_C|GetTraceLength _suspensioncomponent_bp)))
      (Variables|/Game/SuspensionComponent_BP.SuspensionComponent_BP_C|SetTraceLength _suspensioncomponent_bp1 (* _jumpheight (Variables|/Game/SuspensionComponent_BP.SuspensionComponent_BP_C|GetTraceLength _suspensioncomponent_bp1)))
      (Variables|/Game/SuspensionComponent_BP.SuspensionComponent_BP_C|SetTraceLength _suspensioncomponent_bp2 (* _jumpheight (Variables|/Game/SuspensionComponent_BP.SuspensionComponent_BP_C|GetTraceLength _suspensioncomponent_bp2)))
      (Variables|/Game/SuspensionComponent_BP.SuspensionComponent_BP_C|SetTraceLength _suspensioncomponent_bp3 (* _jumpheight (Variables|/Game/SuspensionComponent_BP.SuspensionComponent_BP_C|GetTraceLength _suspensioncomponent_bp3)))
      (Utilities|FlowControl|Delay 5.0)
      (Variables|/Game/SuspensionComponent_BP.SuspensionComponent_BP_C|SetTraceLength _suspensioncomponent_bp (* (Variables|/Game/SuspensionComponent_BP.SuspensionComponent_BP_C|GetTraceLength _suspensioncomponent_bp) _returnvalue))
      (Variables|/Game/SuspensionComponent_BP.SuspensionComponent_BP_C|SetTraceLength _suspensioncomponent_bp1 (* (Variables|/Game/SuspensionComponent_BP.SuspensionComponent_BP_C|GetTraceLength _suspensioncomponent_bp1) _returnvalue))
      (Variables|/Game/SuspensionComponent_BP.SuspensionComponent_BP_C|SetTraceLength _suspensioncomponent_bp2 (* (Variables|/Game/SuspensionComponent_BP.SuspensionComponent_BP_C|GetTraceLength _suspensioncomponent_bp2) _returnvalue))
      (Variables|/Game/SuspensionComponent_BP.SuspensionComponent_BP_C|SetTraceLength _suspensioncomponent_bp3 (* (Variables|/Game/SuspensionComponent_BP.SuspensionComponent_BP_C|GetTraceLength _suspensioncomponent_bp3) _returnvalue))
      (Variables|Default|SetStiltsOn false)
      (goto _label Reset))))

(event Custom|GoForward
  (bind _carmesh (Variables|Default|GetCarMesh))
  (bind _carspeed (Variables|Default|GetCarSpeed))
  (bind _returnvalue (Math|Vector|GetForwardVector _carmesh))
  (bind _returnvalue_2 (* (Math|Vector|MakeVector (.x _returnvalue) (.y _returnvalue) 0.0) _carspeed))
  (bind _returnvalue_3 (* _returnvalue_2 1.0))
  ;[1 1 1] Go Forward (Always happening)
  (Physics|AddForce (Variables|Default|GetCarMesh) (Math|Vector|MakeVector (.x _returnvalue_3) (.y _returnvalue_3) 0.0) "None" false))

(event Custom|AddGravity
  (bind _carmesh (Variables|Default|GetCarMesh))
  (bind _returnvalue (Transformation|GetWorldLocation _carmesh))
  ;[1 1 1] Add artificial gravity
  (bind _outhit (Collision|LineTraceByChannel (Math|Vector|MakeVector (.x _returnvalue) (.y _returnvalue) (.z _returnvalue)) (Math|Vector|MakeVector (.x _returnvalue) (.y _returnvalue) 0.0) "TraceTypeQuery1" false 0 "ForOneFrame"))
  (if (> (.Distance (Collision|BreakHitResult _outhit)) 1e+02)
    (if (not (Variables|Default|GetStiltsOn))
      (Physics|AddImpulse (Variables|Default|GetCarMesh) "0, 0,-1000.000000" "None" false))))

(event Custom|Thruster
  ;[1 1 1] Thruster
  (bind _output_get (Variables|Default|SetCarSpeed (* (Variables|Default|GetCarSpeed) 2.0)))
  (Utilities|FlowControl|Delay 5.0)
  (Variables|Default|SetCarSpeed (* _output_get 0.5)))

(event EventBeginPlay
  (bind _carmesh (Variables|Default|GetCarMesh))
  (Default|InitComponent (Variables|Default|GetSuspensionComponent_BP) _carmesh)
  (Default|InitComponent (Variables|Default|GetSuspensionComponent_BP1) _carmesh)
  (Default|InitComponent (Variables|Default|GetSuspensionComponent_BP2) _carmesh)
  (Default|InitComponent (Variables|Default|GetSuspensionComponent_BP3) _carmesh))

(event EventTick
  (params (DeltaSeconds :type Float%20%28single-precision%29))
  (CallFunction|GoForward)
  (CallFunction|AddGravity)
  (Development|PrintString (Utilities|String|ToString(Float) (.roll (Transformation|GetWorldRotation (Variables|Default|GetCarMesh))))))

(event Input|ActionEvents|InputActionFlip
  (params (Key :type Key%20Structure :default "None"))
  (bind _carmesh (Variables|Default|GetCarMesh))
  (bind _returnvalue (Transformation|GetWorldRotation _carmesh))
  ;[1 1 1] Flip car right side up
  (:Pressed
    (Transformation|SetWorldRotation _carmesh (Math|Rotator|MakeRotator 0.0 (.pitch _returnvalue) (.yaw _returnvalue)) false false)))

(event Input|AxisEvents|InputAxisForward
  (params (AxisValue :type Float%20%28single-precision%29))
  ;[1 1 1] Control for debugging
)

(event Input|AxisEvents|InputAxisTurn
  (params (AxisValue :type Float%20%28single-precision%29))
  ;[1 1 1] Turn Control
  (Class|PrimitiveComponent|AddTorqueinDegrees (Variables|Default|GetCarMesh) (Math|Vector|MakeVector 0.0 0.0 (* AxisValue 1.5e+08)) "None" false))

(fn ConstructionScript)